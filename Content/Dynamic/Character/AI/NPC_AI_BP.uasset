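; AI controller for guard NPCs that loads the patrol blackboard and runs the guard behavior tree on BeginPlay.
; AI Perception updates set the blackboard Enemy key to sensed actors lacking the "Enemy" tag and clear it when sensing fails.
; Behavior tree decorators read that key to decide whether to follow.
; Perception debug printing, a WorldOrigin key write and deprecated aim-and-shoot logic remain unconnected.
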(event OnTargetPerceptionUpdated(AIPerception)
  (params (Actor :type Actor%20Object%20Reference) (Stimulus :type AI%20Stimulus%20Structure))
  ;[1 1 1] 设置跟随敌人行为
  (CallFunction|UpdateBlackboardEnemyKey Stimulus Actor Actor))

(event EventBeginPlay
  (bind _blackboardcomponent (Class|AIController|UseBlackboard "/Game/Dynamic/Character/AI/BlackBoard_PatrolData.BlackBoard_PatrolData"))
  (AI|RunBehaviorTree "/Game/Dynamic/Character/AI/BT_GuardBehaviour.BT_GuardBehaviour")
  (Variables|Default|SetBlackboard%20Comp _blackboardcomponent))

(fn ConstructionScript)

(fn UpdateBlackboardEnemyKey
  (params (AIStimulus :type AI%20Stimulus%20Structure%20%28by%20ref%29) (ObjectValue :type Object%20Object%20Reference) (self2 :type Actor%20Object%20Reference))
  (bind _enemy (Variables|Default|GetEnemy))
  (bind _blackboard_comp (Variables|Default|GetBlackboard%20Comp))
  (if (not (Actor|ActorHasTag self2 "Enemy"))
    (if (.bSuccessfullySensed (Utilities|Struct|BreakAIStimulus AIStimulus))
      (AI|Components|Blackboard|SetValueasObject _blackboard_comp _enemy ObjectValue)
      (else
        (AI|Components|Blackboard|ClearValue _blackboard_comp _enemy) ; 行为树装饰器会根据此数值\n来判断是否跟随
      ))))