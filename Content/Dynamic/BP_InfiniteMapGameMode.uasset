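; Game mode for an infinite tile map that spawns a short run of BP_TileMap actors at startup and keeps the game score.
; BeginPlay fills a NavMeshBoundsVolume pool, then runs a fixed loop that spawns a tile, waits on a delay and increments the score.
; Each tile receives the shared pool and supplies the attach transform where the next one spawns, chaining them end to end.
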(event EventBeginPlay
  (Class|InfiniteMapGameMode|PopulateBoundsVolumePool)
  (for _index (range 0 3)
    (CallFunction|SpawnTiledMap)
    (Utilities|FlowControl|Delay 2.0)
    (CallFunction|IncreaseScore)))

(fn ConstructionScript)

(fn SpawnTiledMap
  (bind _returnvalue (Game|SpawnActorfromClass "/Game/Dynamic/Terrain/BP_TileMap.BP_TileMap_C" (Variables|Default|GetNextTileTransform) "Undefined" 0 0))
  (Class|Tiles|SetPool _returnvalue (Variables|Default|GetNavMeshBoundsVolumePool))
  (bind _attach_transform (Default|GetAttachLocation _returnvalue))
  (Variables|Default|SetNextTileTransform _attach_transform))

(fn IncreaseScore
  (Math|Integer|IncrementInt (Variables|Default|GetGameScore)))

(fn GetGameScore
  (return (Variables|Default|GetGameScore)))