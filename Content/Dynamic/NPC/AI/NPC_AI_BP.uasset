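; AI controller for guard NPCs that runs BT_GuardBehaviour on the BlackBoard_PatrolData blackboard.
; Perception updates store sensed actors lacking the "Enemy" tag in the Enemy key and clear it when sensing fails, which, per its comment, drives the tree's follow decorator.
; Each Tick, the TPCharacter pawn's aiming and shooting states mirror whether a focus actor exists.
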(event OnTargetPerceptionUpdated(AIPerception)
  (params (Actor :type Actor%20Object%20Reference) (Stimulus :type AI%20Stimulus%20Structure))
  (bind _enemy (Variables|Default|GetEnemy))
  (bind _blackboard_comp (Variables|Default|GetBlackboard%20Comp))
  ;[1 1 1] 设置跟随敌人行为
  (if (not (Actor|ActorHasTag Actor "Enemy"))
    (if (.bSuccessfullySensed (Utilities|Struct|BreakAIStimulus Stimulus))
      (AI|Components|Blackboard|SetValueasObject _blackboard_comp _enemy Actor)
      (else
        (AI|Components|Blackboard|ClearValue _blackboard_comp _enemy) ; 行为树装饰器会根据此数值\n来判断是否跟随
      ))))

(event EventBeginPlay
  (bind _blackboardcomponent (Class|AIController|UseBlackboard "/Game/Dynamic/NPC/AI/BlackBoard_PatrolData.BlackBoard_PatrolData"))
  (AI|RunBehaviorTree "/Game/Dynamic/NPC/AI/BT_GuardBehaviour.BT_GuardBehaviour")
  (Variables|Default|SetBlackboard%20Comp _blackboardcomponent))

(event EventTick
  (params (DeltaSeconds :type Float%20%28single-precision%29))
  (bind _returnvalue (Class|AIController|GetFocusActor))
  (bind _returnvalue_2 (Utilities|IsValid _returnvalue))
  (bind _astpcharacter (Utilities|Casting|CastToTPCharacter (Pawn|GetControlledPawn)))
  (Variables|/Game/Dynamic/NPC/Behaviour/TPCharacter.TPCharacter_C|SetAimingState _astpcharacter _returnvalue_2)
  (Variables|/Game/Dynamic/NPC/Behaviour/TPCharacter.TPCharacter_C|SetShootingState _astpcharacter _returnvalue_2))

(fn ConstructionScript)