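; BP_TileMap is one terrain tile of an infinite map, randomly dressed with props and AI enemies on BeginPlay through PlaceActors and PlaceAIPawns.
; LockingVolume opens a red/green barrier wall while the player is inside, relocks on exit, and scores the tile once.
; When the player enters DeletingVolume, the tile asks BP_InfiniteMapGameMode to spawn another tile, then destroys itself.
; GetAttachLocation exposes the Arrow transform as an attach point.
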(event OnComponentBeginOverlap(LockingVolume)
  (params (OverlappedComponent :type Primitive%20Component%20Object%20Reference) (OtherActor :type Actor%20Object%20Reference) (OtherComp :type Primitive%20Component%20Object%20Reference) (OtherBodyIndex :type Integer) (bFromSweep :type Boolean) (SweepResult :type Hit%20Result%20Structure%20%28by%20ref%29))
  (Utilities|IsPlayerActor OtherActor)
  (Utilities|FlowControl|Sequence
    (:then_0
      (CallFunction|Unlock))
    (:then_1
      (CallFunction|MapPassed))))

(event OnComponentEndOverlap(LockingVolume)
  (params (OverlappedComponent :type Primitive%20Component%20Object%20Reference) (OtherActor :type Actor%20Object%20Reference) (OtherComp :type Primitive%20Component%20Object%20Reference) (OtherBodyIndex :type Integer))
  (Utilities|IsPlayerActor OtherActor)
  (CallFunction|Lock))

(event OnComponentBeginOverlap(DeletingVolume)
  (params (OverlappedComponent :type Primitive%20Component%20Object%20Reference) (OtherActor :type Actor%20Object%20Reference) (OtherComp :type Primitive%20Component%20Object%20Reference) (OtherBodyIndex :type Integer) (bFromSweep :type Boolean) (SweepResult :type Hit%20Result%20Structure%20%28by%20ref%29))
  (Utilities|IsPlayerActor OtherActor)
  (bind _asbp_infinite_map_game_mode (Utilities|Casting|CastToBP_InfiniteMapGameMode (Game|GetGameMode)))
  (Default|SpawnTiledMap _asbp_infinite_map_game_mode)
  (Actor|DestroyActor))

(event EventBeginPlay
  (CallFunction|Lock)
  (Utilities|FlowControl|Sequence
    (:then_0
      ;[1 1 1] Barrels
      (Class|Tiles|PlaceActors "/Game/Dynamic/Terrain/Props/BP_SM_Barrel01.BP_SM_Barrel01_C" 1 5 5e+01 1.0 1.0)
      (Class|Tiles|PlaceActors "/Game/Dynamic/Terrain/Props/BP_SM_Barrel02.BP_SM_Barrel02_C" 1 5 5e+01 1.0 1.0)
      (Class|Tiles|PlaceActors "/Game/Dynamic/Terrain/Props/BP_SM_Barrel03.BP_SM_Barrel03_C" 1 5 5e+01 1.0 1.0)
      (Class|Tiles|PlaceActors "/Game/Dynamic/Terrain/Props/BP_SM_Barrel04.BP_SM_Barrel04_C" 1 2 1e+02 1.0 1.0)
      ;[1 1 1] Containers
      (Class|Tiles|PlaceActors "/Game/Dynamic/Terrain/Props/BP_Container_LeftOpen.BP_Container_LeftOpen_C" 1 2 4e+02 1.0 1.0)
      (Class|Tiles|PlaceActors "/Game/Dynamic/Terrain/Props/BP_Container_NoDoor.BP_Container_NoDoor_C" 1 2 4e+02 1.0 1.0)
      (Class|Tiles|PlaceActors "/Game/Dynamic/Terrain/Props/BP_Container_RightHalfOpen.BP_Container_RightHalfOpen_C" 1 2 4e+02 1.0 1.0)
      ;[1 1 1] Rocks
      (Class|Tiles|PlaceActors "/Game/Dynamic/Terrain/Props/BP_Rock01_High.BP_Rock01_High_C" 1 3 1.5e+02 1.0 5.0)
      (Class|Tiles|PlaceActors "/Game/Dynamic/Terrain/Props/BP_Rock05_High.BP_Rock05_High_C" 1 3 2e+02 1.0 5.0)
      (Class|Tiles|PlaceActors "/Game/Dynamic/Terrain/Props/BP_Rock17_High.BP_Rock17_High_C" 1 3 2e+02 1.0 5.0))
    (:then_1
      ;[1 1 1] Paper Boxes
      (Class|Tiles|PlaceActors "/Game/Dynamic/Terrain/Props/BP_SM_CartonBox_NoOpen1.BP_SM_CartonBox_NoOpen1_C" 1 2 6e+01 1.0 1.0)
      (Class|Tiles|PlaceActors "/Game/Dynamic/Terrain/Props/BP_SM_CartonBox_NoOpen2.BP_SM_CartonBox_NoOpen2_C" 1 2 6e+01 1.0 1.0)
      (Class|Tiles|PlaceActors "/Game/Dynamic/Terrain/Props/BP_SM_CartonBox_Opened.BP_SM_CartonBox_Opened_C" 1 1 6e+01 1.0 1.0)
      (Class|Tiles|PlaceActors "/Game/Dynamic/Terrain/Props/BP_SM_CartonGarbage07.BP_SM_CartonGarbage07_C" 1 1 6e+01 1.0 1.0)
      (Class|Tiles|PlaceActors "/Game/Dynamic/Terrain/Props/BP_SM_CartonGarbage08.BP_SM_CartonGarbage08_C" 1 1 6e+01 1.0 1.0)
      (Class|Tiles|PlaceActors "/Game/Dynamic/Terrain/Props/BP_SM_CartonGarbage09.BP_SM_CartonGarbage09_C" 1 1 6e+01 1.0 1.0)
      ;[1 1 1] Green Boxes
      (Class|Tiles|PlaceActors "/Game/Dynamic/Terrain/Props/BP_Boxes.BP_Boxes_C" 1 1 1.5e+02 1.0 1.0)
      (Class|Tiles|PlaceActors "/Game/Dynamic/Terrain/Props/BP_OneBox.BP_OneBox_C" 1 1 1.5e+02 1.0 1.0)
      ;[1 1 1] Wood Boxes
      (Class|Tiles|PlaceActors "/Game/Dynamic/Terrain/Props/BP_SM_Box_HeapUp.BP_SM_Box_HeapUp_C" 1 1 2.5e+02 1.0 1.0)
      (Class|Tiles|PlaceActors "/Game/Dynamic/Terrain/Props/BP_SM_Boxes.BP_SM_Boxes_C" 1 1 2.5e+02 1.0 1.0))
    (:then_2
      ;[1 1 1] Trifles
      (Class|Tiles|PlaceActors "/Game/Dynamic/Terrain/Props/BP_Canister.BP_Canister_C" 1 5 4e+01 1.0 1.0)
      (Class|Tiles|PlaceActors "/Game/Dynamic/Terrain/Props/BP_SackPacks.BP_SackPacks_C" 1 3 2e+02 1.0 1.0)
      (Class|Tiles|PlaceActors "/Game/Dynamic/Terrain/Props/BP_SM_Pallet01.BP_SM_Pallet01_C" 1 2 6e+01 1.0 1.0)
      ;[1 1 1] AI
      (Class|Tiles|PlaceAIPawns "/Game/Dynamic/Character/Behaviour/BP_Character.BP_Character_C" (Variables|Default|GetMinEnemies) (Variables|Default|GetMaxEnemies) 1e+02))))

(fn ConstructionScript)

(fn GetAttachLocation
  (return (Transformation|GetWorldTransform (Variables|Default|GetArrow))))

(fn Unlock
  (Collision|SetCollisionEnabled (Variables|Default|GetWallForLock) "NoCollision")
  (Rendering|Material|SetMaterial (Variables|Default|GetWallForLock) 0 "/Game/Dynamic/Terrain/MI_Barrier_Green.MI_Barrier_Green"))

(fn Lock
  (Collision|SetCollisionEnabled (Variables|Default|GetWallForLock) "QueryAndPhysics")
  (Rendering|Material|SetMaterial (Variables|Default|GetWallForLock) 0 "/Game/Dynamic/Terrain/MI_Barrier_rED.MI_Barrier_Red"))

(fn MapPassed
  (if (not (Variables|Default|GetIsMapPassed))
    (bind _asbp_infinite_map_game_mode (Utilities|Casting|CastToBP_InfiniteMapGameMode (Game|GetGameMode)))
    (Default|IncreaseScore _asbp_infinite_map_game_mode)
    (Variables|Default|SetIsMapPassed true)))